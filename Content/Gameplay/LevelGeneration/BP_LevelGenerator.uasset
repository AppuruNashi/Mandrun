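; Level generator that builds a level along the Y axis from node classes grouped by type in NodeList.
; Generate stores the seed, then spawns a random start node at StartPoint and an end node offset by chunk count and length.
; Picks use random streams seeded by unseeded RandomInteger(InitialSeed), so results are not reproducible per seed.
; Middle chunk spawning is an empty stub, and missing start or end types print errors.
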(event `Generate`
  (params (Seed :type Integer))
  (set `self.InitialSeed` Seed)
  (`self.SpawnStart`)
  (`self.SpawnMiddleChunks`)
  (`self.SpawnEnd`))

(event `SpawnStart`
  (bind (_value _returnvalue) (`BlueprintMapLibrary.Map_Find` (`self.NodeList`) "NewEnumerator0"))
  (if _returnvalue
    (bind _output_get (set `self.ModifiedSeed` (`KismetMathLibrary.RandomInteger` (`self.InitialSeed`))))
    (`|SpawnActorFromClass` (break `/Game/Gameplay/LevelGeneration/Datas/FNodeWeight` (`KismetArrayLibrary.Array_RandomFromStream` (`.List_10_BC2D8C5F4895E1092CB07EB3C1BF8367` (break `/Game/Gameplay/LevelGeneration/Datas/FNodeListByTypes` _value)) (`KismetMathLibrary.MakeRandomStream` _output_get))) (`KismetMathLibrary.MakeTransform` (`KismetMathLibrary.MakeVector` 0.0 (`self.StartPoint`))) "Undefined" "OverrideRootScale" null null)
    (else
      (`KismetSystemLibrary.PrintString` "Error : Missing Start node type in NodeList in BP_LevelGenerator::SpawnStart" true true (struct :`R` 1.0 :`A` 1.0) 10.0))))

(event `SpawnMiddleChunks`)

(event `SpawnEnd`
  (bind (_value _returnvalue) (`BlueprintMapLibrary.Map_Find` (`self.NodeList`) "NewEnumerator1"))
  (if _returnvalue
    (bind _output_get (set `self.ModifiedSeed` (`KismetMathLibrary.RandomInteger` (`self.InitialSeed`))))
    (`|SpawnActorFromClass` (break `/Game/Gameplay/LevelGeneration/Datas/FNodeWeight` (`KismetArrayLibrary.Array_RandomFromStream` (`.List_10_BC2D8C5F4895E1092CB07EB3C1BF8367` (break `/Game/Gameplay/LevelGeneration/Datas/FNodeListByTypes` _value)) (`KismetMathLibrary.MakeRandomStream` _output_get))) (`KismetMathLibrary.MakeTransform` (`KismetMathLibrary.MakeVector` 0.0 (+ (+ (`self.StartPoint`) (* (`self.MaxNumberOfChunks`) (`self.LenghtOfChuncks`))) (`self.LenghtOfChuncks`)))) "Undefined" "OverrideRootScale" null null)
    (else
      (`KismetSystemLibrary.PrintString` "Error : Missing End node type in NodeList in BP_LevelGenerator::SpawnEnd" true true (struct :`R` 1.0 :`A` 1.0) 10.0))))

(fn `UserConstructionScript`)