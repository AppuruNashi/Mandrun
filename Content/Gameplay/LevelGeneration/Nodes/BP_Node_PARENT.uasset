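; Base level-generation node that randomizes its prop actors from the game mode's initial seed at BeginPlay.
; FillArray is an empty hook, apparently for children to populate RandomActorList before Randomize runs.
; Randomize passes each BP_RandomProps_PARENT a chained value from RandomInteger, which takes the previous value as its upper bound rather than using a seeded stream.
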(event `self.ReceiveBeginPlay`
  (bind _asgm_mrgame_mode (cast `/Game/Gameplay/Global/GM_MRGameMode` (`GameplayStatics.GetGameMode`)))
  (`self.FillArray`)
  (bind _output_get (set `self.Seed` (`KismetMathLibrary.BreakRandomStream` (`/Game/Gameplay/Global/GM_MRGameMode.Seed` _asgm_mrgame_mode))))
  (`self.Randomize` _output_get))

(fn `FillArray`)

(fn `Randomize`
  (params (Seed :type Integer))
  (locals (LocalSeed :type Integer))
  (set `local.LocalSeed` Seed)
  (for _array_element (`self.RandomActorList`)
    (set `local.LocalSeed` (`KismetMathLibrary.RandomInteger` (`local.LocalSeed`)))
    (bind _asbp_random_props_parent (cast `/Game/Gameplay/GameplayProps/PropsList/BP_RandomProps_PARENT` _array_element))
    (`/Game/Gameplay/GameplayProps/PropsList/BP_RandomProps_PARENT.Randomize` _asbp_random_props_parent (`local.LocalSeed`))))

(fn `UserConstructionScript`)