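; BP_Node_End_1 is an end-node variant for level generation, built on a parent node Blueprint.
; Its FillArray override calls the parent, then sets RandomActorList to the actors spawned by its two child actor components.
; BeginPlay is disabled and the construction script only calls the parent, so any other behavior comes from the parent class.
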(fn `FillArray`
  (`parent.FillArray`)
  (set `self.RandomActorList` (`|MakeArray` (`ChildActorComponent.ChildActor` (`self.ChildActor`)) (`ChildActorComponent.ChildActor` (`self.ChildActor1`)))))

(fn `UserConstructionScript`
  (`parent.UserConstructionScript`))