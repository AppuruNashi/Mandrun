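; BP_Node_Pot_2 is a pot node variant for level generation, built on a parent node Blueprint.
; It overrides FillArray to call the parent, then set RandomActorList to the actors spawned by its six Child Actor components.
; The construction script only calls the parent, and any logic that uses the list lies outside this Blueprint.
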(fn `FillArray`
  (`parent.FillArray`)
  (set `self.RandomActorList` (`|MakeArray` (`ChildActorComponent.ChildActor` (`self.ChildActor`)) (`ChildActorComponent.ChildActor` (`self.ChildActor3`)) (`ChildActorComponent.ChildActor` (`self.ChildActor4`)) (`ChildActorComponent.ChildActor` (`self.ChildActor2`)) (`ChildActorComponent.ChildActor` (`self.ChildActor1`)) (`ChildActorComponent.ChildActor` (`self.ChildActor5`)))))

(fn `UserConstructionScript`
  (`parent.UserConstructionScript`))