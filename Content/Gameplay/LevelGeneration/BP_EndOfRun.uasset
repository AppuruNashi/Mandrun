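; BP_EndOfRun is the end-of-run actor for level generation, serving as the win trigger and a closing window.
; When the player character overlaps its Box, it calls OnWin on GM_MRGameMode.
; It also binds to the game mode's close-window event, which runs a timeline that scales the frame's starting relative Z to move frame and window together, then plays a closing sound.
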(event `self.ReceiveBeginPlay`
  (bind _asgm_mrgame_mode (cast `/Game/Gameplay/Global/GM_MRGameMode` (`GameplayStatics.GetGameMode`)))
  (add `/Game/Gameplay/Global/GM_MRGameMode.CloseWindow` _asgm_mrgame_mode (`|CreateDelegate` :!event `CloseWindow`))
  (add `PrimitiveComponent.OnComponentBeginOverlap` (`self.Box`) (`|CreateDelegate` :!event `CustomEvent`)))

(event `CloseWindow`
  (bind (_relativelocation_x _relativelocation_y _relativelocation_z) (`KismetMathLibrary.BreakVector` (`SceneComponent.RelativeLocation` (`self.MovingFrame`))))
  (set `self.StartingPosition` _relativelocation_z)
  (bind (_direction _newtrack_0) (`Timeline|Closing` :!via `PlayFromStart`)
    (:`Update`
      (`SceneComponent.K2_SetRelativeLocation` (`self.MovingFrame`) (`KismetMathLibrary.MakeVector` 0.0 0.0 (* _newtrack_0 (`self.StartingPosition`))) false false)
      (`SceneComponent.K2_SetRelativeLocation` (`self.MovingWindow`) (`KismetMathLibrary.MakeVector` 0.0 0.0 (* _newtrack_0 (`self.StartingPosition`))) false false))
    (:`Finished`
      (`GameplayStatics.PlaySoundAtLocation` "/Game/Audio/SoundEffects/S_WindowClosing.S_WindowClosing" (`SceneComponent.K2_GetComponentLocation` (`self.MovingWindow`)) (struct) 1.0 1.0 0.0 null null null null))))

(event `CustomEvent`
  (params (OverlappedComponent :type "PrimitiveComponent Object Reference") (OtherActor :type "Actor Object Reference") (OtherComp :type "PrimitiveComponent Object Reference") (OtherBodyIndex :type Integer) (bFromSweep :type Boolean) (SweepResult :type "HitResult Structure (by ref)"))
  (if (== OtherActor (`GameplayStatics.GetPlayerCharacter` 0))
    (bind _asgm_mrgame_mode (cast `/Game/Gameplay/Global/GM_MRGameMode` (`GameplayStatics.GetGameMode`)))
    (`/Game/Gameplay/Global/GM_MRGameMode.OnWin` _asgm_mrgame_mode)))

(fn `UserConstructionScript`)