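; Parent Blueprint for pot props that the player can use to get potted, showing an interaction marker when nearby.
; A box overlap with the player character toggles the game mode's can-pot state and shows or hides the marker widget.
; While the marker is shown, Tick updates its text from the game mode's IsPotted flag.
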(event `self.ReceiveBeginPlay`
  (add `PrimitiveComponent.OnComponentBeginOverlap` (`self.Box`) (`|CreateDelegate` :!event `PlayerOnPot`))
  (add `PrimitiveComponent.OnComponentEndOverlap` (`self.Box`) (`|CreateDelegate` :!event `PlayerLeavePot`))
  (bind _asgm_mrgame_mode (cast `/Game/Gameplay/Global/GM_MRGameMode` (`GameplayStatics.GetGameMode`)))
  (set `self.Gamemode` _asgm_mrgame_mode))

(event `self.ReceiveTick`
  (params (DeltaSeconds :type "Float (single-precision)"))
  (if (`self.ShowWidget`)
    (bind _aswbp_mrinteraction_marker (cast `/Game/UI/Markers/WBP_MRInteractionMarker` (`WidgetComponent.GetWidget` (`self.Widget`))))
    (`/Game/UI/Markers/WBP_MRInteractionMarker.ChangePotText` _aswbp_mrinteraction_marker (not (`/Game/Gameplay/Global/GM_MRGameMode.bIsPotted` (`self.Gamemode`))))))

(event `PlayerOnPot`
  (params (OverlappedComponent :type "PrimitiveComponent Object Reference") (OtherActor :type "Actor Object Reference") (OtherComp :type "PrimitiveComponent Object Reference") (OtherBodyIndex :type Integer) (bFromSweep :type Boolean) (SweepResult :type "HitResult Structure (by ref)"))
  (if (== (`GameplayStatics.GetPlayerCharacter` 0) OtherActor)
    (set `self.ShowWidget` true)
    (`/Game/Gameplay/Global/GM_MRGameMode.ToggleCanPot` (`self.Gamemode`) true)
    (`SceneComponent.SetHiddenInGame` (`self.Widget`) false false)))

(event `PlayerLeavePot`
  (params (OverlappedComponent :type "PrimitiveComponent Object Reference") (OtherActor :type "Actor Object Reference") (OtherComp :type "PrimitiveComponent Object Reference") (OtherBodyIndex :type Integer))
  (if (== (`GameplayStatics.GetPlayerCharacter` 0) OtherActor)
    (set `self.ShowWidget` false)
    (`/Game/Gameplay/Global/GM_MRGameMode.ToggleCanPot` (`self.Gamemode`) false)
    (`SceneComponent.SetHiddenInGame` (`self.Widget`) true false)))

(fn `UserConstructionScript`
  (`parent.UserConstructionScript`))