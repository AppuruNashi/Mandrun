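; Game mode that manages a run from start to win or loss, plus level changes for restarting or returning to the main menu.
; BeginPlay seeds a random stream after a short delay, then starts the run, signalling its start and timing it on Tick.
; OnWin and OnLose end the run and show their screen with UI-only input and cursor.
; It also stores CanPot and IsPotted flags.
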(event `ToggleCanPot`
  (params (CanPot :type Boolean))
  (set `self.bCanPot` CanPot))

(event `TogglePot`
  (params (IsPotted :type Boolean))
  (set `self.bIsPotted` IsPotted))

(event `self.ReceiveBeginPlay`
  (`KismetSystemLibrary.Delay` 0.1)
  (`KismetMathLibrary.SeedRandomStream` (`self.Seed`))
  (`self.StartRun`))

(event `GoToMainMenu`
  (`GameplayStatics.OpenLevelBySoftObjectPtr` "/Game/Maps/MRMainMenuLevel.MRMainMenuLevel"))

(event `self.ReceiveTick`
  (params (DeltaSeconds :type "Float (single-precision)"))
  (if (`self.bRunInProgress`)
    (set `self.TimeElapsed` (+ (`self.TimeElapsed`) DeltaSeconds))))

(event `RestartRun`
  (bind _returnvalue (`GameplayStatics.GetPlayerController` 0))
  (`GameplayStatics.OpenLevelBySoftObjectPtr` "/Game/Maps/MRMainLevel.MRMainLevel")
  (`WidgetBlueprintLibrary.SetInputMode_GameOnly` _returnvalue :!label _label)
  (set `PlayerController.bShowMouseCursor` false _returnvalue)
  (`self.RunStart`)
  (set `self.TimeElapsed` 0.0)
  (set `self.bRunInProgress` true))

(event `StartRun`
  (goto _label))

(event `EndOfRun`
  (`self.RunEnd`)
  (set `self.bRunInProgress` false))

(event `OnWin`
  (bind _returnvalue (`GameplayStatics.GetPlayerController` 0))
  (`self.EndOfRun`)
  (bind _returnvalue_2 (`|CreateWidget` "/Game/UI/Menus/WBP_MRWinScreen.WBP_MRWinScreen_C" _returnvalue))
  (`UserWidget.AddToViewport` _returnvalue_2 0)
  (`WidgetBlueprintLibrary.SetInputMode_UIOnlyEx` _returnvalue _returnvalue_2)
  (set `PlayerController.bShowMouseCursor` true _returnvalue :!label _label_2))

(event `OnLose`
  (bind _returnvalue (`GameplayStatics.GetPlayerController` 0))
  (`self.EndOfRun`)
  (bind _returnvalue_2 (`|CreateWidget` "/Game/UI/Menus/WBP_MRLoseScreen.WBP_MRLoseScreen_C" _returnvalue))
  (`UserWidget.AddToViewport` _returnvalue_2 0)
  (`WidgetBlueprintLibrary.SetInputMode_UIOnlyEx` _returnvalue _returnvalue_2)
  (goto _label_2))

(fn `UserConstructionScript`)